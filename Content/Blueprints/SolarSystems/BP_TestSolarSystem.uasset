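; BP_TestSolarSystem is a test solar system actor that assembles one sun and two planets from child actor components.
; Its Construction Script sets Sun from the test sun's child actor, then clears and refills the Planets array with the planet child actors that cast successfully to Planet.
; The Event Graph holds only disabled default events, so the Blueprint adds no runtime logic of its own.
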(event EventBeginPlay)

(event Collision|EventActorBeginOverlap
  (params (OtherActor :type Actor%20Object%20Reference)))

(event EventTick
  (params (DeltaSeconds :type Float%20%28single-precision%29)))

(fn ConstructionScript
  (Variables|Default|SetSun (Variables|/Script/Engine.ChildActorComponent|GetChildActor (Variables|Default|GetBP_TestSun)))
  (Utilities|Array|Clear (Variables|Default|GetPlanets))
  (bind _asplanet (Utilities|Casting|CastToPlanet (Variables|/Script/Engine.ChildActorComponent|GetChildActor (Variables|Default|GetBP_TestPlanet1)))
    (:then
      (Utilities|Array|Add (Variables|Default|GetPlanets) _asplanet))
    (:CastFailed
      _))
  (bind _asplanet_2 (Utilities|Casting|CastToPlanet (Variables|/Script/Engine.ChildActorComponent|GetChildActor (Variables|Default|GetBP_TestPlanet2))))
  (Utilities|Array|Add (Variables|Default|GetPlanets) _asplanet_2))